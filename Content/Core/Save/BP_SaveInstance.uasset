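; Game instance that owns the BP_UserSettings save object, loading it on Init or creating it if absent.
; Macros handle player stats (rounding some floats), city info and items, with saves written to the SettingsSave slot.
; It tracks destroyed actors for lookup and can delete the SettingsSave and GameSave slots.
; Player transform save and restore logic exists but is disconnected.
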(event Custom|StoreNameItem
  (params (Item :type Name))
  (Utilities|Array|AddUnique (Variables|Item|GetDestroyedActors) Item))

(event Custom|DeleteItem
  (params (ItemRef :type BP%20Pick%20Item%20Parent%20Object%20Reference))
  (Utilities|Array|AddUnique (Variables|Item|GetItemRef) ItemRef))

(event EventInit
  (CallFunction|LoadUserSettings))

(fn GetUserSettings
  (bind _usersettings (Variables|Default|GetUserSettings)
    (:then
      (return _usersettings))
    (:else
      (CallFunction|LoadUserSettings)
      (return (Variables|Default|GetUserSettings)))))

(fn LoadUserSettings
  (bind _returnvalue (SaveGame|DoesSaveGameExist (Variables|Default|GetSettingsSave)))
  (if _returnvalue
    (bind _returnvalue_2 (SaveGame|LoadGamefromSlot (Variables|Default|GetSettingsSave)))
    (bind _asbp_user_settings (Utilities|Casting|CastToBP_UserSettings _returnvalue_2))
    (Variables|Default|SetUserSettings _asbp_user_settings)
    (|PlayerTransform
      (:OutputPin
        _)
      (:then
        _))
    (|PlayerData
      (:NewParam2
        (|LoadItems
          (:NewParam2
            (Utilities|Struct|SetmembersinF_City (Variables|Default|GetCityInfo) (Utilities|Struct|BreakF_City (Variables|/Game/Core/Save/BP_UserSettings.BP_UserSettings_C|GetCityInfo (Variables|Default|GetUserSettings))))
            (return)))))
    (else
      (bind _returnvalue_3 (SaveGame|CreateSaveGameObject "/Game/Core/Save/BP_UserSettings.BP_UserSettings_C"))
      (Variables|Default|SetUserSettings _returnvalue_3)
      (return))))

(fn SaveSettings
  (Utilities|Struct|SetmembersinF_Gameplay (Variables|Default|GetGameplayeSettings) (Utilities|Struct|BreakF_Gameplay (Variables|/Game/Core/Save/BP_UserSettings.BP_UserSettings_C|GetGameplayInfo (Variables|Default|GetUserSettings))))
  (|SavePlayerData)
  (|SaveItems
    (:NewParam
      (Utilities|Struct|SetmembersinF_City (Variables|Default|GetCityInfo) (Utilities|Struct|BreakF_City (Variables|/Game/Core/Save/BP_UserSettings.BP_UserSettings_C|GetCityInfo (Variables|Default|GetUserSettings))))
      (SaveGame|SaveGametoSlot (Variables|Default|GetUserSettings) (Variables|Default|GetSettingsSave)))))

(fn DeleteSave
  (SaveGame|DeleteGameinSlot (Variables|Default|GetSettingsSave))
  (SaveGame|DeleteGameinSlot (Variables|Default|GetGameSave)))

(fn AddFloats
  (bind _usersettings (Variables|Default|GetUserSettings))
  (bind _playersettings (Variables|/Game/Core/Save/BP_UserSettings.BP_UserSettings_C|GetPlayerSettings _usersettings))
  (bind (_currentexp _neededexp _currenthealth _maxhealth _currentmana _maxmana _durabilityprocent _accuracy _criticalhit _dodging _persuasion _negotiation) (Utilities|Struct|BreakF_PlayerData _playersettings))
  (bind _structout (Utilities|Struct|SetmembersinF_PlayerData (Variables|Default|GetPlayerSettings) (Math|Conversions|ToFloat(Integer) (Math|Float|Round _currentexp)) (Math|Conversions|ToFloat(Integer) (Math|Float|Round _neededexp)) (Math|Conversions|ToFloat(Integer) (Math|Float|Round _currenthealth)) (Math|Conversions|ToFloat(Integer) (Math|Float|Round _maxhealth)) (Math|Conversions|ToFloat(Integer) (Math|Float|Round _currentmana)) (Math|Conversions|ToFloat(Integer) (Math|Float|Round _maxmana)) _durabilityprocent _accuracy _criticalhit _dodging _persuasion _negotiation))
  (return (Utilities|Struct|MakeF_PlayerData (.CurrentEXP (Utilities|Struct|BreakF_PlayerData _structout)) (.NeededEXP (Utilities|Struct|BreakF_PlayerData _structout)) (.CurrentHealth (Utilities|Struct|BreakF_PlayerData _structout)) (.MaxHealth (Utilities|Struct|BreakF_PlayerData _structout)) (.CurrentMana (Utilities|Struct|BreakF_PlayerData _structout)) (.MaxMana (Utilities|Struct|BreakF_PlayerData _structout)) (.DurabilityProcent (Utilities|Struct|BreakF_PlayerData _structout)) (.Accuracy (Utilities|Struct|BreakF_PlayerData _structout)) (.CriticalHit (Utilities|Struct|BreakF_PlayerData _structout)) (.Dodging (Utilities|Struct|BreakF_PlayerData _structout)) (.Persuasion (Utilities|Struct|BreakF_PlayerData _structout)) (.Negotiation (Utilities|Struct|BreakF_PlayerData _structout)))))

(fn CheckifAlreadyDestroyed
  (params (NewParam :type Name))
  (return (> (Utilities|Array|FindItem (Variables|Item|GetDestroyedActors) NewParam) -1)))