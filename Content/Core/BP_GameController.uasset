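; Game controller Blueprint that handles the minimap, pause menu and actor interaction for the player.
; BeginPlay adds the minimap widget and starts a looping timer that line-traces forward from the character's capsule to set or clear FocusedActor.
; The interaction input sends InteractionMessage to that actor.
; Pause input or TogglePause toggles the menu, game pause, cursor and input mode; full-map toggle and settings-save nodes are unconnected.
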(event Input|EnhancedActionEvents|EnhancedInputActionIA_Map
  (params (ActionValue :type Boolean) (ElapsedSeconds :type Float%20%28double-precision%29) (TriggeredSeconds :type Float%20%28double-precision%29) (InputAction :type Input%20Action%20Object%20Reference :default "/Game/Core/Inputs/Movement/IA_Map.IA_Map")))

(event Input|EnhancedActionEvents|EnhancedInputActionIA_Pause
  (params (ActionValue :type Boolean) (ElapsedSeconds :type Float%20%28double-precision%29) (TriggeredSeconds :type Float%20%28double-precision%29) (InputAction :type Input%20Action%20Object%20Reference :default "/Game/Core/Inputs/MenuInputs/IA_Pause.IA_Pause"))
  ;[1 1 1] Pause Menu
  (:Started
    (CallFunction|TogglePauseMenu)))

(event EventBeginPlay
  (bind _returnvalue (UserInterface|CreateWidget "/Game/Widgets/WBP_MiniMap.WBP_MiniMap_C"))
  (UserInterface|Viewport|AddtoViewport _returnvalue 0)
  (CallFunction|Initialize))

(event EventTogglePause
  ;[1 1 1] Pause Menu
  (CallFunction|TogglePauseMenu))

(event Input|EnhancedActionEvents|EnhancedInputActionIA_Interaction
  (params (ActionValue :type Boolean) (ElapsedSeconds :type Float%20%28double-precision%29) (TriggeredSeconds :type Float%20%28double-precision%29) (InputAction :type Input%20Action%20Object%20Reference :default "/Game/Core/Inputs/Default/IA_Interaction.IA_Interaction"))
  (:Started
    (Class|BPIInteraction|Interaction(Message) (Variables|Interaction|GetFocusedActor))))

(fn ConstructionScript)

(fn TogglePauseMenu
  (bind _returnvalue (Game|GetPlayerController 0))
  (if (Variables|Default|GetPauseMenuToggle?)
    (Widget|RemovefromParent (Variables|Default|GetPauseMenuWidget))
    (Game|SetGamePaused false)
    (Variables|Default|SetPauseMenuToggle? false)
    (Variables|/Script/Engine.PlayerController|SetbShowMouseCursor (Game|GetPlayerController 0) false)
    (Input|SetInputModeGameOnly (Game|GetPlayerController 0) false)
    (else
      (bind _returnvalue_2 (UserInterface|CreateWidget "/Game/Widgets/PauseMenu/WBP_PauseMenu.WBP_PauseMenu_C"))
      (bind _output_get (Variables|Default|SetPauseMenuWidget _returnvalue_2))
      (UserInterface|Viewport|AddtoViewport _output_get 0)
      (Game|SetGamePaused true)
      (Variables|Default|SetPauseMenuToggle? true)
      (Variables|/Script/Engine.PlayerController|SetbShowMouseCursor _returnvalue true)
      (Input|SetInputModeGameandUI _returnvalue (Variables|Default|GetPauseMenuWidget) "DoNotLock" false false))))

(fn TraceforInteraction
  (bind _returnvalue (Game|GetPlayerCharacter 0))
  (bind _returnvalue_2 (Actor|GetComponentbyClass _returnvalue "/Script/Engine.CapsuleComponent"))
  (bind _returnvalue_3 (Transformation|GetWorldLocation _returnvalue_2))
  (Utilities|IsValid _returnvalue_2
    (:Is%20Valid
      (Variables|Interaction|SetTraceStart _returnvalue_3)
      (Variables|Interaction|SetTraceEnd (+ _returnvalue_3 (* (Math|Vector|GetForwardVector _returnvalue_2) (Variables|Interaction|GetInteractionDistance))))
      (bind (_outhit _returnvalue_4) (Collision|LineTraceForObjects (Variables|Interaction|GetTraceStart) (Variables|Interaction|GetTraceEnd) (Utilities|Array|MakeArray "ObjectTypeQuery7" "ObjectTypeQuery1") false (Utilities|Array|MakeArray (Game|Player|GetPlayerPawn 0)) "ForOneFrame"))
      (if _returnvalue_4
        (Variables|Interaction|SetFocusedActor (.HitActor (Collision|BreakHitResult _outhit)))
        (else
          (Interaction|ClearFocusedActor))))))

(fn Initialize
  (Utilities|Time|SetTimerbyFunctionName 0 "TraceForInteraction" 0.1 true))

(fn ClearFocusedActor
  (Variables|Interaction|GetFocusedActor
    (:then
      _)
    (:else
      _))
  (Variables|Interaction|SetFocusedActor 0))